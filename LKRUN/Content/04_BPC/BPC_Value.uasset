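; Actor component that holds a clamped bar value, either a posture bar that starts empty or a standard bar that starts full.
; A looping timer applies the recovery value and broadcasts bar updates until the value returns to its resting end.
; AddValue changes the value and, on a hit that stops short of the bar's limit, pauses recovery before a delayed restart.
; ClearTimers cancels both recovery and restart timers.
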(event `self.ReceiveBeginPlay`
  (set `self.Owner` (`self.GetOwner`))
  (set `self.CurrentValue` (select `bool` (`self.IsPostureBar`) :`false` (`self.MaxValue`)))
  (`self.Reco`))

(event `Reco`
  (if (<= (`self.CurrentValue`) (`self.MaxValue`))
    (bind _returnvalue (`KismetSystemLibrary.K2_SetTimerDelegate` (delegate `Recovery`) 0.1 true))
    (set `self.PropertyHandle` _returnvalue)))

(event `Recovery`
  (bind _propertyhandle (`self.PropertyHandle`))
  (if (select `bool` (`self.IsPostureBar`) :`false` (< (`self.CurrentValue`) (`self.MaxValue`)) :`true` (> (`self.CurrentValue`) 0.0))
    (set `self.CurrentValue` (`KismetMathLibrary.FClamp` (+ (`self.CurrentValue`) (`self.CurrentRecoveryValue`)) 0.0 (`self.MaxValue`)))
    (`self.OnUpdateBars`)
    (elif (`KismetSystemLibrary.K2_IsValidTimerHandle` _propertyhandle)
      (`KismetSystemLibrary.K2_ClearAndInvalidateTimerHandle` _propertyhandle))))

(event `ClearTimers`
  (`KismetSystemLibrary.K2_ClearAndInvalidateTimerHandle` (`self.PropertyHandle`))
  (`KismetSystemLibrary.K2_ClearAndInvalidateTimerHandle` (`self.StopHandle`)))

(fn `AddValue`
  (params (Added :type "Float (double-precision)"))
  (returns (CurrentValue :type "Float (double-precision)"))
  (bind _added (`local.Added`))
  (bind _maxvalue (`self.MaxValue`))
  (bind _output_get (set `self.CurrentValue` (`KismetMathLibrary.FClamp` (+ Added (`self.CurrentValue`)) 0.0 _maxvalue)))
  (if (select `bool` (`self.IsPostureBar`) :`false` (< _output_get 1.0) :`true` (> _output_get (- _maxvalue 0.1)))
    (return (`self.CurrentValue`))
    (elif (select `bool` (`self.IsPostureBar`) :`false` (< _added 0.0) :`true` (> _added 0.0))
      (`KismetSystemLibrary.K2_ClearAndInvalidateTimerHandle` (`self.PropertyHandle`))
      (bind _returnvalue (`KismetSystemLibrary.K2_SetTimer` null "Reco" 3.0))
      (set `self.StopHandle` _returnvalue)
      (return (`self.CurrentValue`))
      (else
        (return (`self.CurrentValue`))))))

(fn `GetCurrentValue`
  (returns (CurrentValue :type "Float (double-precision)"))
  (return (`self.CurrentValue`)))