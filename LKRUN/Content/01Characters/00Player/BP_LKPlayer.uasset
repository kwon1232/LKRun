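; BP_LKPlayer is a player character Blueprint with basic axis-driven movement and look controls.
; Turn and LookUp feed controller yaw and pitch, while MoveForward adds movement along the control rotation's forward vector.
; MoveRight is bound but does nothing, as its strafe logic is left disconnected.
; The construction script lowers the mesh by the scaled capsule half-height to align it with the capsule's base.
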(event `InputAxis|Turn`
  (params (AxisValue :type "Float (single-precision)"))
  (`self.AddControllerYawInput` AxisValue))

(event `InputAxis|MoveForward`
  (params (AxisValue :type "Float (single-precision)"))
  (`self.AddMovementInput` (`KismetMathLibrary.GetForwardVector` (`self.GetControlRotation`)) AxisValue))

(event `InputAxis|LookUp`
  (params (AxisValue :type "Float (single-precision)"))
  (`self.AddControllerPitchInput` AxisValue))

(event `InputAxis|MoveRight`
  (params (AxisValue :type "Float (single-precision)")))

(fn `UserConstructionScript`
  (`SceneComponent.K2_SetRelativeLocation` (`self.Mesh`) (`KismetMathLibrary.MakeVector` 0.0 0.0 (- 0.0 (`CapsuleComponent.GetScaledCapsuleHalfHeight` (`self.CapsuleComponent`)))) false false))